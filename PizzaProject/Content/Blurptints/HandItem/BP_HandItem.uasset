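; BP_HandItem is a hand item Blueprint that tracks whether its owner is moving horizontally.
; It caches the owner's location on BeginPlay.
; Each Tick it sets IsMoves from any non-zero XY displacement since the last frame, ignoring vertical movement, then stores the new location.
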(event EventTick
  (params (DeltaSeconds :type Float%20%28single-precision%29))
  (if (> (Math|Vector|VectorLengthXY (- (Transformation|GetActorLocation (Components|GetOwner)) (Variables|Default|GetLastOwnerLocation))) 0.0)
    (Variables|Default|SetIsMoves true)
    (else
      (Variables|Default|SetIsMoves false)))
  (Variables|Default|SetLastOwnerLocation (Transformation|GetActorLocation (Components|GetOwner))))

(event EventBeginPlay
  (Variables|Default|SetLastOwnerLocation (Transformation|GetActorLocation (Components|GetOwner))))